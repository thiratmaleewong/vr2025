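; Cannon Blueprint that aims its barrel and then moves a bomb to a target location in a scripted sequence on BeginPlay.
; It zeroes the Canon component's world rotation, waits briefly, then a timeline interpolates it to Targetrotator.
; When that finishes, it stores the Bomb's current location and a second timeline lerps the bomb to TargetLocation2, without sweep or physics teleport.
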(event EventBeginPlay
  (Transformation|SetWorldRotation (Variables|Default|Getcanon) "0, 0, 0" false false)
  (Variables|Default|Setselfrotator "0, 0, 0")
  (Utilities|FlowControl|Delay 0.2)
  (bind _time (Timeline|Timeline PlayFromStart)
    (:Update
      (Transformation|SetWorldRotation (Variables|Default|Getcanon) (Math|Rotator|Lerp(Rotator) (Variables|Default|Getselfrotator) (Variables|Default|Gettargetrotator) _time) false false))
    (:Finished
      (Variables|Default|SetSelfLocation_2 (Transformation|GetWorldLocation (Variables|Default|Getbomb)))
      (bind _time_2 (Timeline|Timeline_0 PlayFromStart)
        (:Update
          (Transformation|SetWorldLocation (Variables|Default|Getbomb) (Math|Vector|Lerp(Vector) (Variables|Default|GetSelfLocation_2) (Variables|Default|GetTargetLocation_2) _time_2) false false))))))

(fn ConstructionScript)